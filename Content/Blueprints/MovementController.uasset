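; MovementController is a character Blueprint that handles movement and switches control between the PlayerBP and MechBP pawns.
; Input events drive walking, jumping and looking, with gamepad look scaled by turn rate and frame time.
; BeginPlay caches the first actor of each class.
; SwitchPossession makes the controller possess whichever of the two is not player-controlled, checking only the player reference for validity and printing debug strings.
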(event `InputAxis|TurnRate`
  (params (AxisValue :type "Float (single-precision)"))
  ;[1 1 1] Gamepad Movement
  (`self.AddControllerYawInput` (* AxisValue (`self.TurnRateGamepad`) (`GameplayStatics.GetWorldDeltaSeconds`))))

(event `InputAxis|LookUpRate`
  (params (AxisValue :type "Float (single-precision)"))
  ;[1 1 1] Gamepad Movement
  (`self.AddControllerPitchInput` (* AxisValue (`self.TurnRateGamepad`) (`GameplayStatics.GetWorldDeltaSeconds`))))

(event `InputAxis|MoveForward`
  (params (AxisValue :type "Float (single-precision)"))
  ;[1 1 1] KBM movement
  (`self.AddMovementInput` (`self.GetActorForwardVector`) AxisValue))

(event `InputAction|Jump`
  (params (Key :type "Key Structure"))
  ;[1 1 1] KBM movement
  (:`Pressed`
    (`self.Jump`))
  (:`Released`
    (`self.StopJumping`)))

(event `InputAxis|Turn`
  (params (AxisValue :type "Float (single-precision)"))
  ;[1 1 1] KBM movement
  (`self.AddControllerYawInput` AxisValue))

(event `InputAxis|LookUp`
  (params (AxisValue :type "Float (single-precision)"))
  ;[1 1 1] KBM movement
  (`self.AddControllerPitchInput` AxisValue))

(event `InputAxis|MoveRight`
  (params (AxisValue :type "Float (single-precision)"))
  ;[1 1 1] KBM movement
  (`self.AddMovementInput` (`self.GetActorRightVector`) AxisValue))

(event `self.ReceiveBeginPlay`
  (bind _returnvalue (`GameplayStatics.GetActorOfClass` "/Game/Blueprints/MechBP.MechBP_C"))
  (set `self.MechRef` _returnvalue)
  (bind _returnvalue_2 (`GameplayStatics.GetActorOfClass` "/Game/Blueprints/PlayerBP.PlayerBP_C"))
  (bind _output_get (set `self.PlayerBPRef` _returnvalue_2))
  (`/Engine/EditorBlueprintResources/StandardMacros.IsValid` _output_get
    (:`Is Valid`
      (`KismetSystemLibrary.PrintString` "good"))
    (:`Is Not Valid`
      (`KismetSystemLibrary.PrintString` "bad"))))

(event `InputAction|SwitchPossession`
  (params (Key :type "Key Structure"))
  (bind _returnvalue (`self.GetController`))
  (bind _playerbpref (`self.PlayerBPRef`))
  (:`Pressed`
    (`/Engine/EditorBlueprintResources/StandardMacros.IsValid` _playerbpref
      (:`Is Valid`
        (if (`self.IsControlled` _playerbpref)
          (`Controller.Possess` _returnvalue (`self.MechRef`))
          (else
            (`Controller.Possess` _returnvalue (`self.PlayerBPRef`)))))
      (:`Is Not Valid`
        (`KismetSystemLibrary.PrintString` "pain")))))

(fn `UserConstructionScript`)